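; Base player ship character for a 2D space shooter: flies in the XZ plane, faces the mouse cursor and fires from two muzzles.
; Tick drives aiming, Delay-paced firing and the sector countdown; movement burns Fuel, and overlaps enable interactables.
; Damage drains Shields, with DoOnce-gated collision grace; death only prints.
; When time expires, a fuel-costing Jump restores shields, resets position and timer, clears enemies, and refreshes the HUD.
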(event `self.ReceiveBeginPlay`
  ;[1 1 1] Create and add HUD to screen.
  (bind _returnvalue (`|CreateWidget` "/Game/Blueprints/UI/WBP_HUD.WBP_HUD_C"))
  (bind _output_get (set `self.HUD` _returnvalue))
  (`UserWidget.AddToViewport` _output_get 0)
  ;[1 1 1] Handles functions that update the HUD.
  (`self.HUDHandler`))

(event `self.ReceiveTick`
  (params (DeltaSeconds :type "Float (single-precision)"))
  ;[1 1 1] Always make the player face the mouse cursor.
  (`self.FaceMouseCursor`)
  ;[1 1 1] If player is firing, spawn projectiles.
  (`self.ShootProjectilesWhenNeccesary`)
  ;[1 1 1] Handle the timer at the top of the HUD.
  (`self.GameTimer`))

(event `Key|H`
  (params (Key :type "Key Structure"))
  ;[1 1 1] Debugging
  (:`Pressed`
    (bind _asbp_game_mode_base (cast `/Game/Blueprints/BP_GameModeBase` (`GameplayStatics.GetGameMode`)))
    (`/Game/Blueprints/BP_GameModeBase.GameTimerFinished` _asbp_game_mode_base)))

(event `self.CapsuleComponent.OnComponentBeginOverlap`
  (params (OverlappedComponent :type "PrimitiveComponent Object Reference") (OtherActor :type "Actor Object Reference") (OtherComp :type "PrimitiveComponent Object Reference") (OtherBodyIndex :type Integer) (bFromSweep :type Boolean) (SweepResult :type "HitResult Structure (by ref)"))
  ;[1 1 1] If the player overlaps with an actor of the Interactable class.
  (bind _asbp_interactable_base (cast `/Game/Blueprints/Interactables/BP_InteractableBase` OtherActor))
  (set `self.OverlappingInteractable` _asbp_interactable_base)
  (set `self.CanPlayerInteract` true))

(event `self.CapsuleComponent.OnComponentEndOverlap`
  (params (OverlappedComponent :type "PrimitiveComponent Object Reference") (OtherActor :type "Actor Object Reference") (OtherComp :type "PrimitiveComponent Object Reference") (OtherBodyIndex :type Integer))
  ;[1 1 1] If the player stops overlapping with an actor of the Interactable class.
  (cast `/Game/Blueprints/Interactables/BP_InteractableBase` OtherActor)
  (set `self.CanPlayerInteract` false))

(event `ManualCollisionDamageReset`
  ;[1 1 1] If the player collides with any enemy, apply damage.
  ;;[1 1 1] Bug fixing event. This event resets the do once node for collision damage. Before you could be invincible when colliding with enemies once you added a fleet ship.
  (goto _label :!via `Reset`))

(event `self.CapsuleComponent.OnComponentHit`
  (params (HitComponent :type "PrimitiveComponent Object Reference") (OtherActor :type "Actor Object Reference") (OtherComp :type "PrimitiveComponent Object Reference") (NormalImpulse :type "Vector Structure") (Hit :type "HitResult Structure (by ref)"))
  ;[1 1 1] If the player collides with any enemy, apply damage.
  (`/Engine/EditorBlueprintResources/StandardMacros.DoOnce` false :!label _label
    (:`Completed`
      ;;[1 1 1] Did the player collide with an enemy?
      (bind _asbp_enemy_base (cast `/Game/Blueprints/Enemies/BP_EnemyBase` OtherActor)
        (:`then`
          (set `self.HitEnemy` _asbp_enemy_base)
          ;;[1 1 1] Apply damage to player.
          (`GameplayStatics.ApplyDamage` self 20.0)
          ;;[1 1 1] This allows a grace period where the player can't take damage from collisions for the amount of time set in InvincibilityDuration.
          (`KismetSystemLibrary.Delay` (`self.InvincibilityDuration`))
          ;;[1 1 1] Reset Do Once.
          (`self.ManualCollisionDamageReset`))
        (:`CastFailed`
          ;;[1 1 1] Reset Do Once.
          (`self.ManualCollisionDamageReset`))))))

(event `self.ReceiveAnyDamage`
  (params (Damage :type "Float (single-precision)") (DamageType :type "DamageType Object Reference") (InstigatedBy :type "Controller Object Reference") (DamageCauser :type "Actor Object Reference"))
  ;[1 1 1] Event for recieve damage.
  ;;[1 1 1] Subtract damage amount from player Shields.
  (set `self.Shields` (`KismetMathLibrary.FClamp` (- (`self.Shields`) Damage) 0.0 (`self.MaxShields`)))
  (`self.UpdateShields`)
  ;;[1 1 1] If player's Shields equal zero and isn't already dead, then set IsDead to true.
  (if (and (== (`self.Shields`) 0.0) (not (`self.IsDead`)))
    (set `self.IsDead` true)
    (`self.PlayerDeath`)))

(event `ShootProjectilesWhenNeccesary`
  ;[1 1 1] Handles when, where and how projectiles are shot.
  ;;[1 1 1] Is the corresponding InputAction being pressed?
  (if (`self.ShootProjectile`)
    ;;[1 1 1] Give a delay between each shot.
    (`KismetSystemLibrary.Delay` (`self.ProjectileShotDelay`))
    ;;[1 1 1] Spawn projectiles from each turrent on sprite.
    (`|SpawnActorFromClass` "/Game/Blueprints/Actors/BP_PlayerBasicProjectile.BP_PlayerBasicProjectile_C" (`SceneComponent.K2_GetComponentToWorld` (`self.ArrowShot1`)) "Undefined" "OverrideRootScale" null null)
    (`|SpawnActorFromClass` "/Game/Blueprints/Actors/BP_PlayerBasicProjectile.BP_PlayerBasicProjectile_C" (`SceneComponent.K2_GetComponentToWorld` (`self.ArrowShot2`)) "Undefined" "OverrideRootScale" null null)))

(event `GameTimer`
  ;[1 1 1] Handles the Timer for the game.
  ;;[1 1 1] Execute every second.
  (`KismetSystemLibrary.Delay` 1.0)
  ;;[1 1 1] If the current seconds equal zero, then we need to look at the minutes.
  (if (== (`self.CurrentSeconds`) 0)
    ;;[1 1 1] If the current minutes equal zero as well, then that means the timer is finished.
    (if (== (`self.CurrentMinutes`) 0)
      ;;[1 1 1] End of time behavior.
      (bind _asbp_game_mode_base (cast `/Game/Blueprints/BP_GameModeBase` (`GameplayStatics.GetGameMode`)))
      (`/Game/Blueprints/BP_GameModeBase.GameTimerFinished` _asbp_game_mode_base)
      (set `self.CanPlayerJump` true)
      (else
        ;;[1 1 1] If false, set Seconds to 59 and decrement Current Minutes once.
        (set `self.CurrentSeconds` 59)
        (bind _result (`/Engine/EditorBlueprintResources/StandardMacros.DecrementInt` (`self.CurrentMinutes`))
          (:`  `
            (set `self.CurrentMinutes` _result)))))
    (else
      ;;[1 1 1] If false, then we only need to decrement the seconds once.
      (bind _result_2 (`/Engine/EditorBlueprintResources/StandardMacros.DecrementInt` (`self.CurrentSeconds`))
        (:`  `
          (set `self.CurrentSeconds` _result_2))))))

(event `InputAxis|MoveRight`
  (params (AxisValue :type "Float (single-precision)"))
  ;[1 1 1] Handles player movement and consequences of moving.
  ;;[1 1 1] Essentially scales the max fly speed in CharacterMovement by the axis value.
  ;;;[1 1 1] Allows player to move to the right and left.
  (if (> (`self.Fuel`) 0.0)
    (`self.AddMovementInput` (1.0 0.0 0.0) AxisValue)
    ;;[1 1 1] If the player is moving at a particular velocity.
    (if (>= (`KismetMathLibrary.VSize` (`MovementComponent.Velocity` (`self.CharacterMovement`))) (/ (`self.MaxVectorLength`) 2.0))
      ;;[1 1 1] Take fuel away and update the fuel visually on the HUD.
      (set `self.Fuel` (- (`self.Fuel`) (`self.MovementFuelCost`)))
      (`self.UpdateFuel`))))

(event `InputAxis|MoveUp`
  (params (AxisValue :type "Float (single-precision)"))
  ;[1 1 1] Handles player movement and consequences of moving.
  ;;[1 1 1] Essentially scales the max fly speed in CharacterMovement by the axis value.
  ;;;[1 1 1] Allows player to move up and down. I changed the default land movement mode to flying in CharacterMovement for this to work.
  (if (> (`self.Fuel`) 0.0)
    (`self.AddMovementInput` (0.0 0.0 1.0) AxisValue)
    ;;[1 1 1] If the player is moving at a particular velocity.
    (if (>= (`KismetMathLibrary.VSize` (`MovementComponent.Velocity` (`self.CharacterMovement`))) (/ (`self.MaxVectorLength`) 2.0))
      ;;[1 1 1] Take fuel away and update the fuel visually on the HUD.
      (set `self.Fuel` (- (`self.Fuel`) (`self.MovementFuelCost`)))
      (`self.UpdateFuel`))))

(event `InputAction|ShootProjectile`
  (params (Key :type "Key Structure"))
  ;[1 1 1] When the player fires projectiles.
  (:`Pressed`
    (set `self.ShootProjectile` true)
    ;;[1 1 1] Set player sprite to the fire flipbook
    (`PaperFlipbookComponent.SetFlipbook` (`self.Sprite`) (`self.FB_Fire`)))
  (:`Released`
    (set `self.ShootProjectile` false)
    ;;[1 1 1] Set player sprite back to the default idle flipbook
    (`PaperFlipbookComponent.SetFlipbook` (`self.Sprite`) (`self.FB_Idle`))))

(event `InputAction|Interact`
  (params (Key :type "Key Structure"))
  (bind _overlappinginteractable (`self.OverlappingInteractable`))
  (bind _overlappinginteractable_2 (`self.OverlappingInteractable`))
  ;[1 1 1] Input Action for interaction.
  (:`Pressed`
    ;;[1 1 1] Check if the player is able to interact. This variable is set in begin and end overlap events.
    (if (`self.CanPlayerInteract`)
      ;;[1 1 1] Allow interaction to begin within the actor.
      (set `/Game/Blueprints/Interactables/BP_InteractableBase.CanInteractableInteract` true _overlappinginteractable_2)
      ;;[1 1 1] Overrided event to handle interaction for every actor of the Interactable class.
      (`/Game/Blueprints/Interactables/BP_InteractableBase.Interact` _overlappinginteractable_2)))
  (:`Released`
    ;;[1 1 1] Make sure there is an Interactable overlapping with the player. Disable interaction within the actor.
    (`/Engine/EditorBlueprintResources/StandardMacros.IsValid` _overlappinginteractable
      (:`Is Valid`
        (set `/Game/Blueprints/Interactables/BP_InteractableBase.CanInteractableInteract` false _overlappinginteractable)))))

(event `InputAction|Jump`
  (params (Key :type "Key Structure"))
  ;[1 1 1] InputAction for when the game timer runs out and the player decides to jump to the 'next' sector.
  (:`Pressed`
    ;;[1 1 1] This makes sure that the player can only jump when the game timer has ended and that the player has enough fuel to make the jump.
    (if (and (`self.CanPlayerJump`) (> (`self.Fuel`) (`self.JumpFuelCost`)))
      ;;[1 1 1] Spawn the player at the starting location with zero velocity incase the player was moving when they decided to jump.
      (bind _outactors (`GameplayStatics.GetAllActorsOfClass` "/Script/Engine.PlayerStart"))
      (`self.K2_SetActorLocation` self (`self.K2_GetActorLocation` (`|GetArrayItem` _outactors)) false false)
      (set `MovementComponent.Velocity` (0.0 0.0 0.0) (`self.CharacterMovement`))
      ;;[1 1 1] Give the player full health.
      (set `self.Shields` (`self.MaxShields`))
      ;;[1 1 1] Take fuel away.
      (set `self.Fuel` (- (`self.Fuel`) (`self.JumpFuelCost`)))
      ;;[1 1 1] Reset the timer to starting values. This also stops the insurmountable enemy fleet from continuing to warp in.
      (set `self.CurrentMinutes` (`self.DefaultMinutes`))
      (set `self.CurrentSeconds` (`self.DefaultSeconds`))
      ;;[1 1 1] Make sure HUD is updated correctly.
      (`self.HUDHandler`)
      ;;[1 1 1] Destroy all enemies.
      (bind _outactors_2 (`GameplayStatics.GetAllActorsOfClass` "/Game/Blueprints/Enemies/BP_EnemyBase.BP_EnemyBase_C"))
      (for _array_element _outactors_2
        (`self.K2_DestroyActor` _array_element))
      ;;[1 1 1] Destroy all enemy projectiles.
      (bind _outactors_3 (`GameplayStatics.GetAllActorsOfClass` "/Game/Blueprints/Actors/BP_EnemyBasicProjectile.BP_EnemyBasicProjectile_C"))
      (for _array_element_2 _outactors_3
        (`self.K2_DestroyActor` _array_element_2))))
  (:`Released`
    (set `self.CanPlayerJump` false)))

(fn `FaceMouseCursor`
  (bind (_returnvalue_x _returnvalue_y _returnvalue_z) (`KismetMathLibrary.BreakVector` (`SceneComponent.K2_GetComponentLocation` (`self.Sprite`))))
  (bind (_bblockinghit _binitialoverlap _time _distance _location) (`GameplayStatics.BreakHitResult` (`PlayerController.GetHitResultUnderCursorByChannel` (`GameplayStatics.GetPlayerController` 0) "TraceTypeQuery2" true)))
  ;[1 1 1] Get the player to face the mouse cursor on screen.
  ;;[1 1 1] Set player's rotation to face the cursor.
  (`SceneComponent.K2_SetWorldRotation` (`self.Sprite`) (`KismetMathLibrary.MakeRotator` 0.0 (* (+ (`KismetMathLibrary.DegAtan2` (- _returnvalue_x (.x _location)) (- _returnvalue_z (.z _location))) 180.0) -1.0)) false false))

(fn `HUDHandler`
  (`self.UpdateShields`)
  (`self.UpdateFuel`)
  (`self.UpdateShips`))

(fn `PlayerDeath`
  (`KismetSystemLibrary.PrintString` "Player is dead"))

(fn `UpdateCapablePopulation`
  ;[1 1 1] Call function in HUD to update Capable Population value visually.
  (`/Game/Blueprints/UI/WBP_HUD.UpdateCapablePopulation` (`self.HUD`) (`self.CapablePopulation`)))

(fn `UpdateCurrentPopulation`
  ;[1 1 1] Call function in HUD to update Current Population value visually.
  (`/Game/Blueprints/UI/WBP_HUD.UpdateCurrentPopulation` (`self.HUD`) (`self.CurrentPopulation`)))

(fn `UpdateFuel`
  ;[1 1 1] Call function in HUD to update Fuel value visually.
  (`/Game/Blueprints/UI/WBP_HUD.UpdateFuel` (`self.HUD`) (`self.Fuel`) (`self.MaxFuel`)))

(fn `UpdateShields`
  ;[1 1 1] Call function in HUD to update Shields value visually.
  (`/Game/Blueprints/UI/WBP_HUD.UpdateShields` (`self.HUD`) (`self.Shields`) (`self.MaxShields`)))

(fn `UpdateShips`
  ;[1 1 1] Call function in HUD to update Ships value visually.
  (`/Game/Blueprints/UI/WBP_HUD.UpdateShips` (`self.HUD`) (`self.Ships`)))

(fn `UserConstructionScript`
  ;[1 1 1] Reset values to preset starting ones.
  (set `self.Shields` (`self.MaxShields`))
  (set `self.Fuel` (`self.MaxFuel`))
  (set `self.CurrentMinutes` (`self.DefaultMinutes`))
  (set `self.CurrentSeconds` (`self.DefaultSeconds`)))