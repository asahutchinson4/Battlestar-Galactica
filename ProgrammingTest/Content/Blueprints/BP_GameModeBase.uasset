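; Game mode that drives enemy and interactable spawning through spawn zone actors placed in the level.
; On BeginPlay it gathers all enemy zones, shuffles them and starts spawning in a configurable number, then tells every interactable zone to spawn.
; GameTimerFinished makes all enemy zones spawn an overwhelming fleet when time runs out; per its comment, the player Blueprint calls it every tick.
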(event `self.ReceiveBeginPlay`
  ;[1 1 1] Get an array of all Enemy Spawn Zones in the map.
  (bind _outactors (`GameplayStatics.GetAllActorsOfClass` "/Game/Blueprints/Actors/BP_EnemySpawnZone.BP_EnemySpawnZone_C"))
  (set `self.EnemySpawnZones` _outactors)
  ;[1 1 1] Begin the process of spawning at the start of the game.
  (`self.BeginSpawningEnemies`)
  (`self.BeginSpawningInteractables`))

(event `BeginSpawningEnemies`
  ;[1 1 1] Select a desired amount of spawn zones to allow spawning.
  ;;[1 1 1] Get the array of all Enemy Spawn Zones and randomize the array's order.
  (`KismetArrayLibrary.Array_Shuffle` (`self.EnemySpawnZones`))
  ;;[1 1 1] Loop through all the Spawn Zones placed in the map. It is customizable to allow the programmer to chose how many spawn zones they want to allow spawning.
  (for _index (range (`self.DesiredSpawnZones`))
    ;;[1 1 1] Get an item from the array and execute their spawning event.
    (`/Game/Blueprints/Actors/BP_EnemySpawnZone.StartSpawnProcess` (`|GetArrayItem` (`self.EnemySpawnZones`) _index))))

(event `GameTimerFinished`
  ;[1 1 1] An insurmountable enemy fleet warps in to overwhelm the player. Does allow a few seconds for the player to Jump to the next sector and/or gather a few more Interactables. Spawn enemies from every Enemy Spawn Zone in the map without a wait time. This occurs every tick since this event is called in the Event Tick of player BP.
  (for _array_element (`self.EnemySpawnZones`)
    (`/Game/Blueprints/Actors/BP_EnemySpawnZone.GameTimerEndedSpawn` _array_element)))

(event `BeginSpawningInteractables`
  ;[1 1 1] Get all Interactable Spawn Zones and begin spawning process for each one.
  (bind _outactors (`GameplayStatics.GetAllActorsOfClass` "/Game/Blueprints/Actors/BP_InteractableSpawnZone.BP_InteractableSpawnZone_C"))
  (bind _output_get (set `self.InteractableSpawnZones` _outactors))
  (for _array_element _output_get
    (`/Game/Blueprints/Actors/BP_InteractableSpawnZone.SpawnInteractables` _array_element)))

(fn `UserConstructionScript`)