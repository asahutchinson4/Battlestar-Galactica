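; BP_InteractableSpawnZone is an actor that scatters interactables across the game board within its SpawnArea bounds.
; SpawnInteractables loops over the InteractableTypes classes and reads each one's SectorLimit class default to decide how many to spawn.
; Each instance spawns at a random point in the bounding box, and fuel pickups also get IncreaseFuelSpawns called on them.
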(event `SpawnInteractables`
  (bind (_origin _boxextent) (`KismetSystemLibrary.GetComponentBounds` (`self.Spawn Area`)))
  ;[1 1 1] Spawn all interactables randomly across the game board.
  ;;[1 1 1] Get all different types of interactables.
  (for _array_element (`self.InteractableTypes`)
    (bind _asbp_interactable_base (castclass `/Game/Blueprints/Interactables/BP_InteractableBase` _array_element))
    ;;[1 1 1] Loop through how many interactables need to be spawned.
    (for _ (range 1 (+ (`.SectorLimit` (defaults `Object` _asbp_interactable_base)) 1))
      ;;[1 1 1] Spawn this interactable at a random location in the Spawn Area.
      (bind _returnvalue (`|SpawnActorFromClass` _asbp_interactable_base (`KismetMathLibrary.MakeTransform` (`KismetMathLibrary.RandomPointInBoundingBox` _origin _boxextent)) "Undefined" "OverrideRootScale" null null))
      ;[1 1 1] If the spawned actor is Pickup Fuel, call this event.
      (bind _asbp_pickup_fuel (cast `/Game/Blueprints/Interactables/BP_PickupFuel` _returnvalue))
      (`/Game/Blueprints/Interactables/BP_PickupFuel.IncreaseFuelSpawns` _asbp_pickup_fuel))))

(fn `UserConstructionScript`)