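; Fuel pickup interactable that adds fuel to the player, capped at their maximum.
; Overlapping the interaction box stores the player, shows a prompt widget and opens a Gate that lets the inherited Interact event through.
; A successful pickup updates the player's fuel display and destroys the actor, discarding any excess.
; A total exactly equal to the maximum matches neither branch, so nothing is picked up.
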(event `self.ReceiveBeginPlay`
  ;[1 1 1] Create widget and reference.
  (bind _returnvalue (`|CreateWidget` "/Game/Blueprints/UI/WBP_PickupFuel.WBP_PickupFuel_C"))
  (set `self.InteractionWidget` _returnvalue))

(event `self.Interact`
  (bind _player (`self.Player`))
  (bind _player_2 (`self.Player`))
  (bind _player_3 (`self.Player`))
  (bind _returnvalue (+ (`self.FuelToGive`) (`/Game/Blueprints/PlayerFleet/BP_PlayerBase.Fuel` _player)))
  ;[1 1 1] Overridden event from parent.
  ;[1 1 1] Allow interaction.
  (set `self.CanInteractableInteract` true)
  ;[1 1 1] Control execution flow for when to allow interaction.
  (`/Engine/EditorBlueprintResources/StandardMacros.Gate` true :!label _label
    (:`Exit`
      ;[1 1 1] Check if player is full on fuel. This should never happen but just as a safety measure.
      (if (== (`/Game/Blueprints/PlayerFleet/BP_PlayerBase.Fuel` _player_2) (`/Game/Blueprints/PlayerFleet/BP_PlayerBase.MaxFuel` _player_2))
        (`KismetSystemLibrary.PrintString` "Fuel is full")
        (else
          ;[1 1 1] Check if the player has space for new fuel.
          (set `self.NewFuel` _returnvalue)
          (if (< _returnvalue (`/Game/Blueprints/PlayerFleet/BP_PlayerBase.MaxFuel` _player))
            (set `/Game/Blueprints/PlayerFleet/BP_PlayerBase.Fuel` (`self.NewFuel`) (`self.Player`))
            ;[1 1 1] Update the HUD and destroy this actor.
            (`self.InteractionBehavior`)
            (else
              ;[1 1 1] Check if the potential new fuel is greater than what the player can hold.
              (if (> (`self.NewFuel`) (`/Game/Blueprints/PlayerFleet/BP_PlayerBase.MaxFuel` (`self.Player`)))
                ;[1 1 1] Essentially grab the fuel you can and leave the rest.
                (set `/Game/Blueprints/PlayerFleet/BP_PlayerBase.Fuel` (`/Game/Blueprints/PlayerFleet/BP_PlayerBase.MaxFuel` _player_3) _player_3)
                ;[1 1 1] Update the HUD and destroy this actor.
                (`self.InteractionBehavior`)))))))))

(event `self.InteractionBox.OnComponentBeginOverlap`
  (params (OverlappedComponent :type "PrimitiveComponent Object Reference") (OtherActor :type "Actor Object Reference") (OtherComp :type "PrimitiveComponent Object Reference") (OtherBodyIndex :type Integer) (bFromSweep :type Boolean) (SweepResult :type "HitResult Structure (by ref)"))
  ;[1 1 1] When the player overlaps with the box collider, open the gate.
  (bind _asbp_player_base (cast `/Game/Blueprints/PlayerFleet/BP_PlayerBase` OtherActor))
  (set `self.Player` _asbp_player_base)
  ;;[1 1 1] Add widget to screen.
  (`UserWidget.AddToViewport` (`self.InteractionWidget`) 0)
  (goto _label :!via `Open`))

(event `self.InteractionBox.OnComponentEndOverlap`
  (params (OverlappedComponent :type "PrimitiveComponent Object Reference") (OtherActor :type "Actor Object Reference") (OtherComp :type "PrimitiveComponent Object Reference") (OtherBodyIndex :type Integer))
  ;[1 1 1] When the player stops overlapping with the box collider, close the gate.
  (cast `/Game/Blueprints/PlayerFleet/BP_PlayerBase` OtherActor)
  ;;[1 1 1] Prevent all interaction.
  (set `self.CanInteractableInteract` false)
  ;;[1 1 1] Remove widget from screen.
  (`Widget.RemoveFromParent` (`self.InteractionWidget`))
  (goto _label :!via `Close`))

(fn `InteractionBehavior`
  (`/Game/Blueprints/PlayerFleet/BP_PlayerBase.UpdateFuel` (`self.Player`))
  (`self.K2_DestroyActor`))

(fn `UserConstructionScript`
  (`parent.UserConstructionScript`))