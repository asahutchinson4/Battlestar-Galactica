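; Fleetship pickup that the player collects by holding interact, adding a ship, max shields and population capacity at a higher movement fuel cost.
; Box overlap shows the interaction widget and opens a gate for the parent's Interact event.
; A retriggerable delay times the hold while a recursive timer poll updates widget progress.
; On completion it destroys itself, updates player stats, widens the HUD shield bar and resets collision damage.
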(event `self.ReceiveBeginPlay`
  ;[1 1 1] Create widget and reference.
  (bind _returnvalue (`|CreateWidget` "/Game/Blueprints/UI/WBP_PlayerFleetship.WBP_PlayerFleetship_C"))
  (set `self.InteractionWidget` _returnvalue))

(event `self.Interact`
  ;[1 1 1] Interaction handling.
  ;;[1 1 1] Overridden event from parent.
  ;;[1 1 1] Allow interaction.
  (set `self.CanInteractableInteract` true)
  ;;[1 1 1] Control execution flow for when to allow interaction.
  (`/Engine/EditorBlueprintResources/StandardMacros.Gate` true :!label _label
    (:`Exit`
      (`|ExecutionSequence`
        (:`then_0`
          ;;[1 1 1] This delay allows the delay to restart if the player lets go of the interact input and then clicks it again.
          (`KismetSystemLibrary.RetriggerableDelay` (`self.MaxHoldTime`))
          ;;[1 1 1] Make sure this actor is able to interact.
          (if (`self.CanInteractableInteract`)
            ;;[1 1 1] Handles what happens when the player interacts with a Fleetship.
            (`self.InteractionBehavior`)))
        (:`then_1`
          ;;[1 1 1] Begin timer and update its value.
          (`self.StartTimer`)
          (`self.UpdateTimer`))))))

(event `self.InteractionBox.OnComponentBeginOverlap`
  (params (OverlappedComponent :type "PrimitiveComponent Object Reference") (OtherActor :type "Actor Object Reference") (OtherComp :type "PrimitiveComponent Object Reference") (OtherBodyIndex :type Integer) (bFromSweep :type Boolean) (SweepResult :type "HitResult Structure (by ref)"))
  (bind _interactionwidget (`self.InteractionWidget`))
  ;[1 1 1] Interaction handling.
  ;;[1 1 1] When the player overlaps with the box collider, open the gate.
  (bind _asbp_player_base (cast `/Game/Blueprints/BP_PlayerBase` OtherActor))
  (set `self.Player` _asbp_player_base)
  ;;;[1 1 1] Set how long the interact button should be held.
  (set `/Game/Blueprints/UI/WBP_PlayerFleetship.MaxTimeHeld` (`self.MaxHoldTime`) _interactionwidget)
  ;;;[1 1 1] Add widget to screen.
  (`UserWidget.AddToViewport` _interactionwidget 0)
  (goto _label :!via `Open`))

(event `self.InteractionBox.OnComponentEndOverlap`
  (params (OverlappedComponent :type "PrimitiveComponent Object Reference") (OtherActor :type "Actor Object Reference") (OtherComp :type "PrimitiveComponent Object Reference") (OtherBodyIndex :type Integer))
  ;[1 1 1] Interaction handling.
  ;;[1 1 1] When the player stops overlapping with the box collider, close the gate.
  (cast `/Game/Blueprints/BP_PlayerBase` OtherActor)
  ;;;[1 1 1] Remove widget from screen.
  (`Widget.RemoveFromParent` (`self.InteractionWidget`))
  ;;;[1 1 1] Stop all interaction.
  (set `self.CanInteractableInteract` false)
  (`self.StopTimer`)
  (set `/Game/Blueprints/UI/WBP_PlayerFleetship.TimeHeld` 0.0 (`self.InteractionWidget`))
  (goto _label :!via `Close`))

(event `StartTimer`
  ;[1 1 1] Timer events.
  ;;[1 1 1] Start timer with set duration.
  (bind _returnvalue (`KismetSystemLibrary.K2_SetTimerDelegate` (delegate `StartTimer`) (`self.MaxHoldTime`)))
  (set `self.InteractionTimer` _returnvalue))

(event `StopTimer`
  ;[1 1 1] Timer events.
  ;;[1 1 1] Stop timer.
  (`KismetSystemLibrary.K2_PauseTimerHandle` (`self.InteractionTimer`)))

(event `UpdateTimer`
  ;[1 1 1] Timer events.
  ;;[1 1 1] Event for handling timer
  ;;;[1 1 1] Check if interaction is allowed.
  (if (`self.CanInteractableInteract`)
    ;;;[1 1 1] Assign widget value to the time that has passed on the timer.
    (set `/Game/Blueprints/UI/WBP_PlayerFleetship.TimeHeld` (`KismetSystemLibrary.K2_GetTimerElapsedTimeHandle` (`self.InteractionTimer`)) (`self.InteractionWidget`))
    ;;;[1 1 1] A slight delay only to prevent an infinite loop from occurring since we are using recursion.
    (`KismetSystemLibrary.Delay` 0.1)
    ;;;[1 1 1] Recursively call this function.
    (`self.UpdateTimer`)
    (else
      ;;;[1 1 1] Stop timer and reset interaction time.
      (`self.StopTimer`)
      (set `/Game/Blueprints/UI/WBP_PlayerFleetship.TimeHeld` 0.0 (`self.InteractionWidget`)))))

(fn `InteractionBehavior`
  (bind _player (`self.Player`))
  (bind _player_2 (`self.Player`))
  (bind _player_3 (`self.Player`))
  (bind _player_4 (`self.Player`))
  (bind _player_5 (`self.Player`))
  ;[1 1 1] Destroy ship.
  (`self.K2_DestroyActor`)
  ;[1 1 1] Increase fuel cost for player.
  (set `/Game/Blueprints/BP_PlayerBase.MovementFuelCost` (+ (`/Game/Blueprints/BP_PlayerBase.MovementFuelCost` _player_3) (`self.ShieldFuelCost`)) _player_3)
  ;[1 1 1] Increase Max Shields for player.
  (set `/Game/Blueprints/BP_PlayerBase.MaxShields` (+ (`/Game/Blueprints/BP_PlayerBase.MaxShields` _player_4) 20.0) _player_4)
  ;[1 1 1] Adjust the appearance of the ShieldsBar on the HUD.
  (bind _output_get (set `self.HUDShieldsBar` (`/Game/Blueprints/UI/WBP_HUD.PlayerShieldsBar` (`/Game/Blueprints/BP_PlayerBase.HUD` (`self.Player`)))))
  (bind _rendertransform (`Widget.RenderTransform` _output_get))
  (bind (_x _y) (`KismetMathLibrary.BreakVector2D` (break `WidgetTransform` _rendertransform)))
  ;[1 1 1] Slightly move the bar. When you scale something it moves so this is to make up for the movement the bar does.
  (`Widget.SetRenderTranslation` (`self.HUDShieldsBar`) (`KismetMathLibrary.MakeVector2D` (+ _x 37.0) _y))
  ;[1 1 1] Scale the bar to be bigger on the x-axis.
  (`Widget.SetRenderScale` (`self.HUDShieldsBar`) (`KismetMathLibrary.MakeVector2D` (+ (`KismetMathLibrary.BreakVector2D` (`.Scale` (break `WidgetTransform` _rendertransform))) 0.2) (`.Y` (`KismetMathLibrary.BreakVector2D` (`.Scale` (break `WidgetTransform` _rendertransform))))))
  ;[1 1 1] Bug fixer: This event resets the do once node for collision damage. Before you could be invincible when colliding with enemies once you added a fleet ship.
  (`/Game/Blueprints/BP_PlayerBase.ManualCollisionDamageReset` (`self.Player`))
  ;[1 1 1] Increase Ships.
  (set `/Game/Blueprints/BP_PlayerBase.Ships` (+ (`/Game/Blueprints/BP_PlayerBase.Ships` _player) 1) _player)
  ;[1 1 1] Increase Capable Population.
  (set `/Game/Blueprints/BP_PlayerBase.CapablePopulation` (+ (`/Game/Blueprints/BP_PlayerBase.CapablePopulation` _player_2) (`/Game/Blueprints/BP_PlayerBase.ShipCapacity` _player_2)) _player_2)
  ;[1 1 1] Update visual representations on the HUD.
  (`/Game/Blueprints/BP_PlayerBase.UpdateShips` _player_5)
  (`/Game/Blueprints/BP_PlayerBase.UpdateShields` _player_5)
  (`/Game/Blueprints/BP_PlayerBase.UpdateCapablePopulation` _player_5))

(fn `InteractionEvent`)

(fn `UserConstructionScript`
  (`parent.UserConstructionScript`))