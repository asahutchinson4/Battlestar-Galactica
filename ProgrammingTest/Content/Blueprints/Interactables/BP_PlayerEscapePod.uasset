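; Interactable escape pod that lets the player rescue a random number of survivors into the fleet's population.
; Box overlap shows a prompt widget and opens a Gate that lets the inherited Interact event through.
; Interact adds survivors if below capacity, clamping any overflow; an exact fill matches neither branch and does nothing.
; A successful rescue checks for the win population, updates the HUD and destroys the pod.
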(event `self.ReceiveBeginPlay`
  ;[1 1 1] Create widget and reference.
  (bind _returnvalue (`|CreateWidget` "/Game/Blueprints/UI/WBP_PlayerEscapePod.WBP_PlayerEscapePod_C"))
  (set `self.InteractionWidget` _returnvalue))

(event `self.Interact`
  (bind _player (`self.Player`))
  (bind _player_2 (`self.Player`))
  (bind _player_3 (`self.Player`))
  ;[1 1 1] Interaction handling.
  ;;[1 1 1] Overridden event from parent.
  ;;[1 1 1] Allow interaction.
  (set `self.CanInteractableInteract` true)
  ;;[1 1 1] Control execution flow for when to allow interaction.
  (`/Engine/EditorBlueprintResources/StandardMacros.Gate` true :!label _label
    (:`Exit`
      ;;[1 1 1] Check if there is any room available in your fleet. True means you are at max capacity.
      (if (not (== (`/Game/Blueprints/PlayerFleet/BP_PlayerBase.CurrentPopulation` _player_3) (`/Game/Blueprints/PlayerFleet/BP_PlayerBase.CapablePopulation` _player_3)))
        ;;[1 1 1] Check if the possible population is less than the allowed amount.
        (bind _output_get (set `self.NewPopulation` (+ (`/Game/Blueprints/PlayerFleet/BP_PlayerBase.CurrentPopulation` _player) (`KismetMathLibrary.RandomIntegerInRange` 3 (`/Game/Blueprints/PlayerFleet/BP_PlayerBase.ShipCapacity` _player)))))
        (if (< _output_get (`/Game/Blueprints/PlayerFleet/BP_PlayerBase.CapablePopulation` _player))
          ;;[1 1 1] Make the population the player currently has the new found population.
          (set `/Game/Blueprints/PlayerFleet/BP_PlayerBase.CurrentPopulation` (`self.NewPopulation`) (`self.Player`))
          ;;[1 1 1] Update the HUD and destroy this actor.
          (`self.InteractionBehavior`)
          (else
            ;;[1 1 1] Check if the New Population is greater than the allowed amount.
            (if (> (`self.NewPopulation`) (`/Game/Blueprints/PlayerFleet/BP_PlayerBase.CapablePopulation` (`self.Player`)))
              ;;[1 1 1] Essentially just save who you can and leave the rest.
              (set `/Game/Blueprints/PlayerFleet/BP_PlayerBase.CurrentPopulation` (`/Game/Blueprints/PlayerFleet/BP_PlayerBase.CapablePopulation` _player_2) _player_2)
              ;;[1 1 1] Update the HUD and destroy this actor.
              (`self.InteractionBehavior`))))))))

(event `self.InteractionBox.OnComponentBeginOverlap`
  (params (OverlappedComponent :type "PrimitiveComponent Object Reference") (OtherActor :type "Actor Object Reference") (OtherComp :type "PrimitiveComponent Object Reference") (OtherBodyIndex :type Integer) (bFromSweep :type Boolean) (SweepResult :type "HitResult Structure (by ref)"))
  ;[1 1 1] Interaction handling.
  ;;[1 1 1] When the player overlaps with the box collider, open the gate.
  (bind _asbp_player_base (cast `/Game/Blueprints/PlayerFleet/BP_PlayerBase` OtherActor))
  (set `self.Player` _asbp_player_base)
  ;;;[1 1 1] Add widget to screen.
  (`UserWidget.AddToViewport` (`self.InteractionWidget`) 0)
  (goto _label :!via `Open`))

(event `self.InteractionBox.OnComponentEndOverlap`
  (params (OverlappedComponent :type "PrimitiveComponent Object Reference") (OtherActor :type "Actor Object Reference") (OtherComp :type "PrimitiveComponent Object Reference") (OtherBodyIndex :type Integer))
  ;[1 1 1] Interaction handling.
  ;;[1 1 1] When the player stops overlapping with the box collider, close the gate.
  (cast `/Game/Blueprints/PlayerFleet/BP_PlayerBase` OtherActor)
  ;;;[1 1 1] Prevent all interaction.
  (set `self.CanInteractableInteract` false)
  ;;;[1 1 1] Remove widget from screen.
  (`Widget.RemoveFromParent` (`self.InteractionWidget`))
  (goto _label :!via `Close`))

(fn `InteractionBehavior`
  (bind _player (`self.Player`))
  ;[1 1 1] Check if the player is qualified to be crowned winner.
  (if (== (`/Game/Blueprints/PlayerFleet/BP_PlayerBase.CurrentPopulation` _player) (`/Game/Blueprints/PlayerFleet/BP_PlayerBase.WinPopulation` _player))
    ;[1 1 1] Execute victory behavior.
    (`/Game/Blueprints/PlayerFleet/BP_PlayerBase.PlayerWon` (`self.Player`)))
  ;[1 1 1] Update HUD and destroy this actor.
  (`/Game/Blueprints/PlayerFleet/BP_PlayerBase.UpdateCurrentPopulation` (`self.Player`))
  (`self.K2_DestroyActor`))

(fn `UserConstructionScript`
  (`parent.UserConstructionScript`))