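; BP_EnemyBase is the base enemy Blueprint, providing AI startup, shield-based damage and a death hook.
; On BeginPlay its AI controller runs the BT_AI behavior tree, while construction resets Shields to DefaultShields.
; AnyDamage subtracts from the clamped Shields, and at zero sets IsDead so death triggers only once.
; EnemyDeath is an empty function that child classes override with their own death logic.
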(event `self.ReceiveBeginPlay`
  ;[1 1 1] Run BT for the enemy logic.
  (`AIController.RunBehaviorTree` (`AIBlueprintHelperLibrary.GetAIController` self) "/Game/AI/Trees/BT_AI.BT_AI"))

(event `self.ReceiveAnyDamage`
  (params (Damage :type "Float (single-precision)") (DamageType :type "DamageType Object Reference") (InstigatedBy :type "Controller Object Reference") (DamageCauser :type "Actor Object Reference"))
  ;[1 1 1] Event for recieve damage.
  ;;[1 1 1] Subtract damage amount from enemy Shields.
  (set `self.Shields` (`KismetMathLibrary.FClamp` (- (`self.Shields`) Damage) 0.0 (`self.DefaultShields`)))
  ;;[1 1 1] If enemy's Shields equal zero and isn't already dead, then set IsDead to true.
  (if (and (== (`self.Shields`) 0.0) (not (`self.IsDead`)))
    (set `self.IsDead` true)
    ;;[1 1 1] Handle the enemy's death.
    (`self.EnemyDeath`)))

(fn `EnemyDeath`
  ;[1 1 1] Overrided: Child specific code here...
)

(fn `UserConstructionScript`
  ;[1 1 1] Reset Shields to the preset value.
  (set `self.Shields` (`self.DefaultShields`)))