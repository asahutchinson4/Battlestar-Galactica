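; BP_EnemySpawnZone is an enemy spawn area that releases a random wave of enemies after a random delay.
; StartSpawnProcess sets a one-shot timer, and SpawnEnemies then spawns a random count of shuffled enemy types at random points inside the SpawnArea bounds.
; After each wave it calls SpawnEnemies on BP_GameModeBase, whose comment says this picks a new zone, and ClearTimer cancels a pending wave.
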(event `StartSpawnProcess`
  ;[1 1 1] An adversity condition that spawns a random set of enemies after a random amount of time.
  ;;[1 1 1] Calculate an Enemy Spawn Time between set range.
  (bind _output_get (set `self.EnemySpawnTime` (`KismetMathLibrary.RandomFloatInRange` (`self.MinEnemySpawnTime`) (`self.MaxEnemySpawnTime`))))
  ;;[1 1 1] When time has elapsed, exectue Spawn Enemies event.
  (bind _returnvalue (`KismetSystemLibrary.K2_SetTimerDelegate` (delegate `SpawnEnemies`) _output_get))
  (set `self.Timer` _returnvalue))

(event `SpawnEnemies`
  (bind (_origin _boxextent) (`KismetSystemLibrary.GetComponentBounds` (`self.Spawn Area`)))
  ;[1 1 1] An adversity condition that spawns a random set of enemies after a random amount of time.
  ;;[1 1 1] Spawn a random enemy type at a random point within the Spawn Area.
  ;;;[1 1 1] For loop that will loop through a desired amount of times.
  (for _ (range 1 (+ (`KismetMathLibrary.RandomIntegerInRange` (`self.MinEnemies`) (`self.MaxEnemies`)) 1))
    ;;;[1 1 1] Randomized an array of all the different enemies in the game. Spawn the enemy that is at particular index at a random point in the Spawn Area.
    (`KismetArrayLibrary.Array_Shuffle` (`self.AllEnemyTypes`))
    (`|SpawnActorFromClass` (`|GetArrayItem` (`self.AllEnemyTypes`)) (`KismetMathLibrary.MakeTransform` (`KismetMathLibrary.RandomPointInBoundingBox` _origin _boxextent)) "Undefined" "OverrideRootScale" null null))
  ;;[1 1 1] Once a wave of enemies has spawned, tell GameMode that its time pick a new and random spawn zone.
  (bind _asbp_game_mode_base (cast `/Game/Blueprints/BP_GameModeBase` (`GameplayStatics.GetGameMode`)))
  (`/Game/Blueprints/BP_GameModeBase.SpawnEnemies` _asbp_game_mode_base))

(event `ClearTimer`
  (`KismetSystemLibrary.K2_ClearAndInvalidateTimerHandle` (`self.Timer`)))

(fn `UserConstructionScript`)